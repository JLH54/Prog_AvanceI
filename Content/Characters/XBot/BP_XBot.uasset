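; BP_XBot is a player-controllable character Blueprint that handles basic movement and camera look through Enhanced Input.
; On BeginPlay it adds IMC_Default to the local player's input subsystem.
; IA_Move feeds movement input along control-rotation right and forward vectors, though the forward direction passes only its Y and Z components.
; IA_Look drives controller yaw and pitch, scaled by LookSpeed and world delta seconds.
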(event `self.ReceiveBeginPlay`
  (bind _asplayer_controller (cast `PlayerController` (`self.GetController`)))
  (`EnhancedInputSubsystemInterface.AddMappingContext` (pcsubsystem `EnhancedInputLocalPlayerSubsystem` _asplayer_controller) "/Game/Input/IMC_Default.IMC_Default" 0 (struct)))

(event `EnhancedInput|/Game/Input/Action/IA_Move`
  (params (ActionValue :type "Vector2D Structure") (ElapsedSeconds :type "Float (double-precision)") (TriggeredSeconds :type "Float (double-precision)") (InputAction :type "InputAction Object Reference" :default "/Game/Input/Action/IA_Move.IA_Move"))
  (bind (_returnvalue_x _returnvalue_y _returnvalue_z) (`KismetMathLibrary.BreakVector` (`KismetMathLibrary.GetForwardVector` (`self.GetControlRotation`))))
  (:`Triggered`
    (`self.AddMovementInput` (`KismetMathLibrary.GetRightVector` (`self.GetControlRotation`)) ActionValue_X)
    (`self.AddMovementInput` (`KismetMathLibrary.MakeVector` 0.0 _returnvalue_y _returnvalue_z) ActionValue_Y)))

(event `EnhancedInput|/Game/Input/Action/IA_Look`
  (params (ActionValue :type "Vector2D Structure") (ElapsedSeconds :type "Float (double-precision)") (TriggeredSeconds :type "Float (double-precision)") (InputAction :type "InputAction Object Reference" :default "/Game/Input/Action/IA_Look.IA_Look"))
  (bind _returnvalue (* (`GameplayStatics.GetWorldDeltaSeconds`) (`self.LookSpeed`)))
  (:`Triggered`
    (`self.AddControllerYawInput` (* ActionValue_X _returnvalue))
    (`self.AddControllerPitchInput` (* ActionValue_Y _returnvalue))))

(fn `UserConstructionScript`)