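; BP_FirstActor is an Actor Blueprint with simple rotation and acceleration functions, none of which currently run.
; RotateFirstActor yaws the actor by delta time times RotationSpeed, while RotateSphere turns the Sphere component by a fixed step per call.
; GoFaster raises Speed over time while it is below MaxSpeed and prints it, but no shown rotation reads Speed.
; BeginPlay, Tick and the construction script are empty, leaving all three function calls unwired.
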(event `self.ReceiveTick`
  (params (DeltaSeconds :type "Float (single-precision)")))

(fn `GoFaster`
  (params (DeltaTime :type "Float (double-precision)"))
  (locals (MaxSpeed :type "Float (double-precision)" :default 500.0) (IncSpeed :type "Float (double-precision)" :default 50.0))
  (if (< (`self.Speed`) (`local.MaxSpeed`))
    (bind _output_get (set `self.Speed` (+ (`self.Speed`) (* DeltaTime (`local.IncSpeed`)))))
    (`KismetSystemLibrary.PrintString` (`KismetStringLibrary.Conv_DoubleToString` _output_get))))

(fn `Rotate First Actor`
  (params (A :type "Float (double-precision)"))
  (`self.K2_AddActorLocalRotation` (`KismetMathLibrary.MakeRotator` 0.0 0.0 (* A (`self.RotationSpeed`)))))

(fn `Rotate Sphere`
  (`SceneComponent.K2_AddLocalRotation` (`self.Sphere`) (struct :`Yaw` 10.0) false false))

(fn `UserConstructionScript`)