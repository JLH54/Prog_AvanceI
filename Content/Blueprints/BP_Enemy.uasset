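; BP_Enemy is an enemy Blueprint with a health bar whose visibility follows its health.
; BeginPlay hides the Healthbar at full health.
; OnUpdateHealth shows it, including at full health, and hides it only when health is exactly zero below maximum.
; Helper functions rotate the actor by a scaled RotationSpeed and the Sphere by a fixed step, but none are called here, and GoFaster is empty.
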(event `self.ReceiveBeginPlay`
  (bind _returnvalue (`self.GetHealth`))
  (bind _returnvalue_2 (`self.GetMaxHealth`))
  (`self.GetPercentHealth`)
  (`SceneComponent.SetVisibility` (`self.Healthbar`) (not (>= _returnvalue _returnvalue_2)) false))

(event `self.OnUpdateHealth`
  (bind _healthbar (`self.Healthbar`))
  (bind _returnvalue (`self.GetHealth`))
  (bind _returnvalue_2 (`self.GetMaxHealth`))
  (if (>= _returnvalue _returnvalue_2)
    (`SceneComponent.SetVisibility` _healthbar true false)
    (else
      (`SceneComponent.SetVisibility` _healthbar (not (== _returnvalue 0.0)) false))))

(fn `GoFaster`
  (params (DeltaTime :type "Float (double-precision)"))
  (locals (MaxSpeed :type "Float (double-precision)" :default 500.0) (IncSpeed :type "Float (double-precision)" :default 50.0)))

(fn `Rotate First Actor`
  (params (A :type "Float (double-precision)"))
  (`self.K2_AddActorLocalRotation` (`KismetMathLibrary.MakeRotator` 0.0 0.0 (* A (`self.RotationSpeed`)))))

(fn `Rotate Sphere`
  (`SceneComponent.K2_AddLocalRotation` (`self.Sphere`) (struct :`Yaw` 10.0) false false))

(fn `UserConstructionScript`)