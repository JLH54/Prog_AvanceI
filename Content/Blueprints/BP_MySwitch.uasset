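; BP_MySwitch is a switch that the player can activate to trigger a linked actor.
; Its box overlaps notify the switch when an Avatar_Player enters or leaves the interaction zone and call CanInteract on the HUD's Master in both cases.
; Activate checks that ActorToInteract implements IInteractable and the switch is unpressed, then calls Pressed, sends DoInteractionMessage to that actor and plays a button sound.
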(event `self.Box.OnComponentBeginOverlap`
  (params (OverlappedComponent :type "PrimitiveComponent Object Reference") (OtherActor :type "Actor Object Reference") (OtherComp :type "PrimitiveComponent Object Reference") (OtherBodyIndex :type Integer) (bFromSweep :type Boolean) (SweepResult :type "HitResult Structure (by ref)"))
  (bind _asavatar_player (cast `Avatar_Player` OtherActor))
  (`self.OnEnterInteractionZone` _asavatar_player)
  (bind _asplayer_controller (cast `PlayerController` (`Pawn.GetController` _asavatar_player)))
  (bind _asbp_hud (cast `/Game/UI/BP_HUD` (`PlayerController.GetHUD` _asplayer_controller)))
  (`/Game/UI/WBP_Master.CanInteract` (`/Game/UI/BP_HUD.Master` _asbp_hud)))

(event `self.Box.OnComponentEndOverlap`
  (params (OverlappedComponent :type "PrimitiveComponent Object Reference") (OtherActor :type "Actor Object Reference") (OtherComp :type "PrimitiveComponent Object Reference") (OtherBodyIndex :type Integer))
  (bind _asavatar_player (cast `Avatar_Player` OtherActor))
  (`self.OnExitInteractionZone` _asavatar_player)
  (bind _asplayer_controller (cast `PlayerController` (`Pawn.GetController` _asavatar_player)))
  (bind _asbp_hud (cast `/Game/UI/BP_HUD` (`PlayerController.GetHUD` _asplayer_controller)))
  (`/Game/UI/WBP_Master.CanInteract` (`/Game/UI/BP_HUD.Master` _asbp_hud)))

(event `self.Activate`
  (if (`KismetSystemLibrary.DoesImplementInterface` (`self.ActorToInteract`) "/Game/Blueprints/IInteractable.IInteractable_C")
    (bind _returnvalue (`self.hasBeenPressed`))
    (if (not _returnvalue)
      (`self.pressed`)
      (message `/Game/Blueprints/IInteractable.DoInteraction` (`self.ActorToInteract`))
      (`GameplayStatics.PlaySoundAtLocation` "/Game/Assets/Audio/UI/Button1.Button1" (`self.K2_GetActorLocation`) (struct) 1.0 1.0 0.0 null null null null))))

(fn `UserConstructionScript`)