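; BP_Switch is an interactable switch that relays the player's activation to another actor.
; A Box component tells Avatar_Player characters entering or leaving it, via OnEnterInteractionZone and OnExitInteractionZone.
; Activate checks that ActorToInteract is valid and implements IInteractable, then calls DoInteractionMessage on it, keeping the switch decoupled from its target's class.
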(event `self.Box.OnComponentBeginOverlap`
  (params (OverlappedComponent :type "PrimitiveComponent Object Reference") (OtherActor :type "Actor Object Reference") (OtherComp :type "PrimitiveComponent Object Reference") (OtherBodyIndex :type Integer) (bFromSweep :type Boolean) (SweepResult :type "HitResult Structure (by ref)"))
  (bind _asavatar_player (cast `Avatar_Player` OtherActor))
  (`self.OnEnterInteractionZone` _asavatar_player))

(event `self.Box.OnComponentEndOverlap`
  (params (OverlappedComponent :type "PrimitiveComponent Object Reference") (OtherActor :type "Actor Object Reference") (OtherComp :type "PrimitiveComponent Object Reference") (OtherBodyIndex :type Integer))
  (bind _asavatar_player (cast `Avatar_Player` OtherActor))
  (`self.OnExitInteractionZone` _asavatar_player))

(event `self.Activate`
  (bind _actortointeract (`self.ActorToInteract`))
  (`/Engine/EditorBlueprintResources/StandardMacros.IsValid` _actortointeract
    (:`Is Valid`
      (if (`KismetSystemLibrary.DoesImplementInterface` _actortointeract "/Game/Blueprints/IInteractable.IInteractable_C")
        (message `/Game/Blueprints/IInteractable.DoInteraction` _actortointeract)))))

(fn `UserConstructionScript`)